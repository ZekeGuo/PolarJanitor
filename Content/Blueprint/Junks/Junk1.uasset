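; Junk1 is a collectible piece of junk that gets sucked toward the player's cleaner.
; It caches the ThirdPersonCharacter on BeginPlay, then checks every Tick whether that character is within range with the cleaner active.
; If so, it restarts a Timeline whose updates move it toward the player using VInterpTo plus a track offset.
; After a short delay it destroys itself, adds its Weight to the player's CurrentGarbageWeight and prints the total.
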(event `self.ReceiveBeginPlay`
  ;[1 1 1] Set the player
  (bind _asthird_person_character (cast `/Game/Blueprint/ThirdPersonBP/Blueprints/ThirdPersonCharacter` (`GameplayStatics.GetPlayerPawn` 0)))
  (set `self.PlayerCharacter` _asthird_person_character))

(event `self.ReceiveTick`
  (params (DeltaSeconds :type "Float (single-precision)"))
  ;[1 1 1] Junk run to cleaner
  (if (<= (`self.GetDistanceTo` (`self.PlayerCharacter`)) 350.0)
    (if (`/Game/Blueprint/ThirdPersonBP/Blueprints/ThirdPersonCharacter.IsCleanerActive` (`self.PlayerCharacter`))
      (bind (_direction _newtrack_2) (`Timeline|Timeline_0` :!via `PlayFromStart`)
        (:`Update`
          (`self.K2_SetActorLocation` (+ _newtrack_2 (`KismetMathLibrary.VInterpTo` (.location (`self.GetTransform`)) (`self.K2_GetActorLocation` (`GameplayStatics.GetPlayerCharacter` 0)) (`GameplayStatics.GetWorldDeltaSeconds`) 6.0)))
          ;[1 1 1] Junk self-destruction & update the junk weight in player's side
          (`KismetSystemLibrary.Delay` 0.2)
          (`self.K2_DestroyActor`)
          (bind _output_get (set `/Game/Blueprint/ThirdPersonBP/Blueprints/ThirdPersonCharacter.Current Garbage Weight` (+ (`/Game/Blueprint/ThirdPersonBP/Blueprints/ThirdPersonCharacter.Current Garbage Weight` (`self.PlayerCharacter`)) (`self.Weight`)) (`self.PlayerCharacter`)))
          (`KismetSystemLibrary.PrintString` (`KismetStringLibrary.Conv_DoubleToString` _output_get)))))))

(fn `UserConstructionScript`)